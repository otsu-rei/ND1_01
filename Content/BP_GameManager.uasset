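; BP_GameManager runs the rules of a Breakout level: block count, ball stock, clear and game over.
; It counts added and broken blocks, showing the clear widget when none remain, and the game-over widget on a miss with no balls left and no clear.
; Action spawns a ball, reloads the level after game over, or opens the next level when cleared.
; Remaining balls carry between levels through BP_BreakoutGameInstance, plus one on each clear.
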(event EventBeginPlay
  (bind _asbp_breakout_game_instance (Utilities|Casting|CastToBP_BreakoutGameInstance (Game|GetGameInstance)))
  (bind _isvalidballnum (Default|IsValidBallNum _asbp_breakout_game_instance))
  (if _isvalidballnum
    (Variables|Default|SetLeftBallNum (Variables|/Game/BP_BreakoutGameInstance.BP_BreakoutGameInstance_C|GetLeftBallNum _asbp_breakout_game_instance))))

(fn ConstructionScript)

(fn AddBlockNum
  (bind _result (Math|Integer|IncrementInt (Variables|Default|GetBlockNum))
    (:%20%20
      (Development|PrintString (Utilities|String|Append "AddBlockNum" (Utilities|String|ToString(Integer) _result)) true true "(R=0.000000,G=0.660000,B=1.000000,A=1.000000)" 1e+01 "AddBlockNum"))))

(fn AddBrokenBlockNum
  (bind _result (Math|Integer|IncrementInt (Variables|Default|GetBrokenBlockNum))
    (:%20%20
      (Development|PrintString (Utilities|String|Append "BrokenBlockNum" (Utilities|String|ToString(Integer) _result)) true true "(R=0.000000,G=0.139141,B=1.000000,A=1.000000)" 1e+01 "BrokenBlockNum")
      (bind _leftblocknum (CallFunction|GetLeftBlockNum))
      (Development|PrintString (Utilities|String|Append "LeftBlockNum" (Utilities|String|ToString(Integer) _leftblocknum)) true true "(R=0.121727,G=0.000000,B=1.000000,A=1.000000)" 1e+01 "LeftBlockNum")
      (bind _leftblocknum_2 (CallFunction|GetLeftBlockNum))
      (if (== _leftblocknum_2 0)
        (CallFunction|ViewGameClearWidget)
        (Variables|Default|SetIsClear true)))))

(fn GetLeftBlockNum
  (return (- (Variables|Default|GetBlockNum) (Variables|Default|GetBrokenBlockNum))))

(fn ViewGameClearWidget
  (bind _returnvalue (UserInterface|CreateWidget "/Game/WBP_GameClear.WBP_GameClear_C"))
  (UserInterface|Viewport|AddtoViewport _returnvalue 0))

(fn ViewGameOverWidget
  (bind _returnvalue (UserInterface|CreateWidget "/Game/WBP_GameOver.WBP_GameOver_C"))
  (UserInterface|Viewport|AddtoViewport _returnvalue 0))

(fn MissCount
  (Variables|Default|SetIsBallSpawned false)
  (if (and (== (Variables|Default|GetLeftBallNum) 0) (not (Variables|Default|GetIsClear)))
    (CallFunction|ViewGameOverWidget)
    (Variables|Default|SetIsGameOver true)))

(fn SpawnBall
  (if (and (not (Variables|Default|GetIsBallSpawned)) (!= (Variables|Default|GetLeftBallNum) 0))
    (Game|SpawnActorfromClass "/Game/BP_Ball.BP_Ball_C" (Math|Transform|MakeTransform (Transformation|GetActorLocation (Variables|Default|GetSpawnLocationActor)) "0, 0, 0" "1.000000,1.000000,1.000000") "Undefined" "MultiplyWithRoot" 0 0)
    (Variables|Default|SetIsBallSpawned true)
    (bind _result (Math|Integer|DecrementInt (Variables|Default|GetLeftBallNum))
      (:%20%20
        (Variables|Default|SetLeftBallNum _result)))))

(fn GetLeftBallNum
  (return (Variables|Default|GetLeftBallNum)))

(fn LevelReset
  (bind _returnvalue (Game|GetCurrentLevelName true))
  (Game|OpenLevel(byName) (Utilities|String|StringToName _returnvalue)))

(fn Action
  (if (Variables|Default|GetIsGameOver)
    (CallFunction|LevelReset)
    (elif (Variables|Default|GetIsClear)
      (CallFunction|OpenNextLevel)
      (else
        (CallFunction|SpawnBall)))))

(fn OpenNextLevel
  (bind _asbp_breakout_game_instance (Utilities|Casting|CastToBP_BreakoutGameInstance (Game|GetGameInstance)))
  (Variables|/Game/BP_BreakoutGameInstance.BP_BreakoutGameInstance_C|SetLeftBallNum _asbp_breakout_game_instance (+ (Variables|Default|GetLeftBallNum) 1))
  (Game|OpenLevel(byName) (Variables|Default|GetNextLevelName)))