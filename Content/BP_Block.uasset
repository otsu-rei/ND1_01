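; BP_Block is a breakable block that loses one HP per Hit event and destroys itself at zero.
; It reports to BP_GameManager on BeginPlay and when broken, so the manager can count total and broken blocks.
; The construction script creates a dynamic material on the cube, and ReloadHp updates the HP text and sets BaseColor from a color table indexed by remaining HP.
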(event Collision|EventHit
  (params (MyComp :type Primitive%20Component%20Object%20Reference) (Other :type Actor%20Object%20Reference) (OtherComp :type Primitive%20Component%20Object%20Reference) (bSelfMoved :type Boolean) (HitLocation :type Vector :default "0, 0, 0") (HitNormal :type Vector :default "0, 0, 0") (NormalImpulse :type Vector :default "0, 0, 0") (Hit :type Hit%20Result%20Structure%20%28by%20ref%29))
  (bind _result (Math|Integer|DecrementInt (Variables|Default|GetHp))
    (:%20%20
      (if (== _result 0)
        (Actor|DestroyActor)
        (bind _returnvalue (Actor|GetActorOfClass "/Game/BP_GameManager.BP_GameManager_C"))
        (Default|AddBrokenBlockNum _returnvalue)
        (else
          (CallFunction|ReloadHp))))))

(event EventBeginPlay
  (bind _returnvalue (Actor|GetActorOfClass "/Game/BP_GameManager.BP_GameManager_C"))
  (Default|AddBlockNum _returnvalue)
  (CallFunction|ReloadHp))

(fn ConstructionScript
  (bind _returnvalue (Rendering|Material|CreateDynamicMaterialInstance (Variables|Default|GetCube) 0 "/Game/M_Block.M_Block" "None" :!class /Script/Engine.PrimitiveComponent))
  (Variables|Default|SetMaterialInstance _returnvalue))

(fn ReloadHp
  (bind _colortable (Variables|Default|GetColorTable))
  (bind _hp (Variables|Default|GetHp))
  (bind _returnvalue (- _hp 1))
  (Rendering|Components|TextRender|SetText (Variables|Default|GetTextRender) (Utilities|Text|ToText(Integer) (Variables|Default|GetHp)))
  (if (Utilities|Array|IsValidIndex _colortable _returnvalue)
    (Rendering|Material|SetVectorParameterValue (Variables|Default|GetMaterialInstance) "BaseColor" (Math|Conversions|ToLinearColor(Color) (Utilities|Array|Get(acopy) _colortable _returnvalue)) :!class /Script/Engine.MaterialInstanceDynamic)))