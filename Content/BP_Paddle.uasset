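; Player-controlled paddle that slides sideways with a swept move via Enhanced Input and forwards the action press to BP_GameManager.
; GetTopNormal fakes a curved top: upward hit normals are rolled in proportion to the hit's Y offset from center, up to a maximum tilt, while other normals pass through unchanged.
; Every tick, it draws debug arrows across the top surface to visualize those tilted normals.
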(event Input|EnhancedActionEvents|EnhancedInputActionIA_Move
  (params (ActionValue :type Float%20%28double-precision%29) (ElapsedSeconds :type Float%20%28double-precision%29) (TriggeredSeconds :type Float%20%28double-precision%29) (InputAction :type Input%20Action%20Object%20Reference :default "/Game/IA_Move.IA_Move"))
  (Transformation|SetActorLocation (+ (* (* (* ActionValue (Class|KismetMathLibrary|VectorRight)) (Variables|Default|GetSpeed)) (Utilities|Time|GetWorldDeltaSeconds)) (Transformation|GetActorLocation)) true false))

(event Input|EnhancedActionEvents|EnhancedInputActionIA_Action
  (params (ActionValue :type Boolean) (ElapsedSeconds :type Float%20%28double-precision%29) (TriggeredSeconds :type Float%20%28double-precision%29) (InputAction :type Input%20Action%20Object%20Reference :default "/Game/IA_Action.IA_Action"))
  (:Started
    (Default|Action (Variables|Default|GetGameManager))))

(event EventBeginPlay
  (Input|AddMappingContext (PlayerController|LocalPlayerSubsystems|GetEnhancedInputLocalPlayerSubsystem (Game|GetPlayerController 0)) "/Game/IMC_InGame.IMC_InGame" 0 "(bIgnoreAllPressedKeysUntilRelease=True,bForceImmediately=False,bNotifyUserSettings=False)")
  (bind _returnvalue (Actor|GetActorOfClass "/Game/BP_GameManager.BP_GameManager_C"))
  (Variables|Default|SetGameManager _returnvalue))

(event EventTick
  (params (DeltaSeconds :type Float%20%28single-precision%29))
  (CallFunction|DrawDebugTopSurfaceNormals))

(fn ConstructionScript)

(fn GetTopNormal
  (params (HitLocation :type Vector) (Normal :type Vector))
  (bind (_origin _boxextent) (Collision|GetActorBounds false false))
  (if (Class|KismetMathLibrary|NotEqualExactlyVectorVector Normal (Math|Vector|VectorUp))
    (return false Normal)
    (else
      (return true (Math|Vector|RotateVector Normal (Math|Rotator|MakeRotator (* (/ (- (.Y (Math|Vector|BreakVector HitLocation)) (.y _origin)) (.y _boxextent)) (Variables|Default|GetMaxTiltNormalDeg)) 0.0 0.0))))))

(fn DrawDebugAllow
  (params (Origin :type Vector) (Direction :type Vector))
  (LocalVariables|SetL_ShapedDirection (* (Math|Vector|Normalize Direction) (LocalVariables|GetL_Length)))
  (Rendering|Debug|DrawDebugArrow Origin (+ Origin (LocalVariables|GetL_ShapedDirection)) 1e+02 "(R=1.000000,G=0.046014,B=0.733476,A=1.000000)" 0.0 1e+01))

(fn DrawDebugTopSurfaceNormals
  (bind (_origin _boxextent) (Collision|GetActorBounds false false))
  (for _index (range (* (LocalVariables|GetL_DrawNumHalf) -1) (LocalVariables|GetL_DrawNumHalf))
    (bind _outnormal (CallFunction|GetTopNormal (+ (Math|Vector|MakeVector 0.0 (* (/ (.y _boxextent) (LocalVariables|GetL_DrawNumHalf)) _index) (.z _boxextent)) _origin) (Math|Vector|VectorUp)))
    (CallFunction|DrawDebugAllow (+ (Math|Vector|MakeVector 0.0 (* (/ (.y _boxextent) (LocalVariables|GetL_DrawNumHalf)) _index) (.z _boxextent)) _origin) _outnormal)))